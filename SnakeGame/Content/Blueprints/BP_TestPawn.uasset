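; BP_TestPawn is a test pawn that spins its controller's view and reports the result.
; Every Tick it adds a constant yaw input and prints the current control rotation to show the change.
; An unconnected chain, which never runs, would set the control rotation to look along negative world forward from the pawn's location.
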(event `self.ReceiveTick`
  (params (DeltaSeconds :type "Float (single-precision)"))
  (`self.AddControllerYawInput` 1.0)
  (`KismetSystemLibrary.PrintString` (`KismetStringLibrary.Conv_RotatorToString` (`self.GetControlRotation`))))

(fn `UserConstructionScript`)