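; Test Blueprint, likely a player controller, that paints a grass compression brush into a deformation render target and previews it on screen.
; BeginPlay clears the target, feeds it into a dynamic UI material shown through WBP_Page, then opens a canvas draw context.
; Tick draws the brush material at full target size on that canvas, which stays open across frames until EndPlay closes it.
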(event `self.ReceiveBeginPlay`
  (`|ExecutionSequence`
    (:`then_0`
      (`KismetRenderingLibrary.ClearRenderTarget2D` (`self.RenderTargetDeformation`) (struct)))
    (:`then_1`
      (bind _returnvalue (`KismetMaterialLibrary.CreateDynamicMaterialInstance` "/Game/Test/M_UI_TestRenderTarget.M_UI_TestRenderTarget"))
      (bind _output_get (set `self.UIMaterial` _returnvalue))
      (`MaterialInstanceDynamic.SetTextureParameterValue` _output_get "RenderTargetTexture" (`self.RenderTargetDeformation`)))
    (:`then_2`
      (bind _returnvalue_2 (`|CreateWidget` "/Game/Test/WBP_Page.WBP_Page_C"))
      (`UserWidget.AddToViewport` _returnvalue_2 0)
      (`/Game/Test/WBP_Page.Set Render Material` _returnvalue_2 _output_get))
    (:`then_4`
      (bind (_canvas _size _context) (`KismetRenderingLibrary.BeginDrawCanvasToRenderTarget` (`self.RenderTargetDeformation`)))
      (set `self.Size` _size)
      (set `self.Context` _context)
      (set `self.Canvas` _canvas))))

(event `self.ReceiveTick`
  (params (DeltaSeconds :type "Float (single-precision)"))
  (`Canvas.K2_DrawMaterial` (`self.Canvas`) "/Game/Test/M_GrassCompressionBrush.M_GrassCompressionBrush" (0.0 0.0) (`self.Size`) (0.0 0.0) (1.0 1.0) 0.0 (0.5 0.5)))

(event `self.ReceiveEndPlay`
  (params (EndPlayReason :type "EEndPlayReason Enum" :default "Destroyed"))
  (`KismetRenderingLibrary.EndDrawCanvasToRenderTarget` (`self.Context`)))

(fn `UserConstructionScript`)