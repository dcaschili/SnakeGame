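; BP_TestPC is a test Blueprint, apparently a player controller, for prototyping grass deformation through a render target, with most of its logic currently disconnected.
; Only EndPlay does work, ending a canvas draw context that no live path begins.
; Unwired chains would clear RenderTargetDeformation, preview it in a WBP_Page widget via a dynamic material, and draw M_GrassCompressionBrush into it through Canvas.
; BeginPlay and Tick are empty.
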(event `self.ReceiveBeginPlay`)

(event `self.ReceiveTick`
  (params (DeltaSeconds :type "Float (single-precision)")))

(event `self.ReceiveEndPlay`
  (params (EndPlayReason :type "EEndPlayReason Enum" :default "Destroyed"))
  (`KismetRenderingLibrary.EndDrawCanvasToRenderTarget` (`self.Context`)))

(fn `UserConstructionScript`)